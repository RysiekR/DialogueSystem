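; Blacksmith NPC dialogue component with time-of-day lines and a small bread-request quest in the afternoon.
; OpenConversation reads hours from the interacting third-person character and selects the Morning, Afternoon or Night branch.
; Dialogue chains AddDialogue nodes by state and option, clearing or rewinding progress on exit so talks restart or resume.
; Accepting the handover sets HasGivenBread, changing later afternoon dialogue; the player's bread check is hardcoded true.
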(fn `Dialogue`
  (`parent.Dialogue`)
  (switch `name` (`self.ActiveDialogueBranch`)
    (:`Morning`
      (bind _state (`self.AddDialogue` "Blacksmith" "good morning" (`|MakeArray`)))
      (switch `/Game/Dialogue/DialogueSystemComponents/Enum_DialogueState` _state
        (:`NewEnumerator0`
          (`self.ClearDialogueProgress`)
          (`self.CloseConversation`))))
    (:`Afternoon`
      (if (`self.bHasGivenBread`)
        (bind _state_2 (`self.AddDialogue` "Blacksmith" "thank you for the bread" (`|MakeArray`)))
        (switch `/Game/Dialogue/DialogueSystemComponents/Enum_DialogueState` _state_2
          (:`NewEnumerator0`
            (`self.ClearDialogueProgress`)
            (`self.CloseConversation`)))
        (else
          (bind (_state_3 _optionindex) (`self.AddDialogue` "Blacksmith" "i would love a piece of bread, can you get me one?" (`|MakeArray` "sure" "no" :!type "Text")))
          (switch `/Game/Dialogue/DialogueSystemComponents/Enum_DialogueState` _state_3
            (:`NewEnumerator0`
              (switch `int` _optionindex
                (:`0`
                  (bind _state_4 (`self.AddDialogue` "Blacksmith" "great, come speak with me when you have it" (`|MakeArray`)))
                  (switch `/Game/Dialogue/DialogueSystemComponents/Enum_DialogueState` _state_4
                    (:`NewEnumerator0`
                      (if true
                        (bind (_state_5 _optionindex_2) (`self.AddDialogue` "Blacksmith" "ahh i see you have bread, can i have it please" (`|MakeArray` "sure" "no" :!type "Text")))
                        (switch `/Game/Dialogue/DialogueSystemComponents/Enum_DialogueState` _state_5
                          (:`NewEnumerator0`
                            (switch `int` _optionindex_2
                              (:`0`
                                (bind _state_6 (`self.AddDialogue` "Blacksmith" "ohh ok so wonderfull i love it" (`|MakeArray`)))
                                (switch `/Game/Dialogue/DialogueSystemComponents/Enum_DialogueState` _state_6
                                  (:`NewEnumerator0`
                                    (`self.ClearDialogueProgress`)
                                    (`self.CloseConversation`))
                                  (:`NewEnumerator1`
                                    (set `self.bHasGivenBread` true))))
                              (:`1`
                                (bind _state_7 (`self.AddDialogue` "Blacksmith" "ohh ok speak to me if you change your mind" (`|MakeArray`)))
                                (switch `/Game/Dialogue/DialogueSystemComponents/Enum_DialogueState` _state_7
                                  (:`NewEnumerator0`
                                    (`self.RemoveDialogueProgress` 2)
                                    (`self.CloseConversation`)))))))
                        (else
                          (bind _state_8 (`self.AddDialogue` "Blacksmith" "come speak with me when you have it" (`|MakeArray`)))
                          (switch `/Game/Dialogue/DialogueSystemComponents/Enum_DialogueState` _state_8
                            (:`NewEnumerator0`
                              (`self.RemoveDialogueProgress` 1)
                              (`self.CloseConversation`))))))))
                (:`1`
                  (bind _state_9 (`self.AddDialogue` "Blacksmith" "ahhh ok speak to me if you change your mind" (`|MakeArray`)))
                  (switch `/Game/Dialogue/DialogueSystemComponents/Enum_DialogueState` _state_9
                    (:`NewEnumerator0`
                      (`self.ClearDialogueProgress`)
                      (`self.CloseConversation`))))))))))
    (:`Night`
      (bind _state_10 (`self.AddDialogue` "Blacksmith" "i am trying to sleep, leave me alone" (`|MakeArray`)))
      (switch `/Game/Dialogue/DialogueSystemComponents/Enum_DialogueState` _state_10
        (:`NewEnumerator0`
          (`self.ClearDialogueProgress`)
          (`self.CloseConversation`))))))

(fn `OpenConversation`
  (bind _instigator (message `/Game/Dialogue/Blueprints/BPI_Interactable.GetInteractInstigator` (`self.GetOwner`)))
  (bind _asbp_third_person_character (cast `/Game/ThirdPerson/Blueprints/BP_ThirdPersonCharacter` _instigator))
  (bind (_timeofday_days _timeofday_hours) (`KismetMathLibrary.BreakTimespan` (`/Game/ThirdPerson/Blueprints/BP_ThirdPersonCharacter.TimeOfDay` _asbp_third_person_character)))
  (`self.SetDialogueBranch` (select `int` (+ (`KismetMathLibrary.Conv_BoolToInt` (and (>= _timeofday_hours 5) (< _timeofday_hours 15))) (* (`KismetMathLibrary.Conv_BoolToInt` (and (>= _timeofday_hours 15) (< _timeofday_hours 22))) 2)) :`0` "Night" :`1` "Morning" :`2` "Afternoon" :`3` "Default" :!type "Name"))
  (`parent.OpenConversation`))