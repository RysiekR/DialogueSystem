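; Test harness component for the quest journal, exercising quest, stage and requirement functions and printing the results to verify them.
; On BeginPlay it gets player 0's journal via GetJournalMessage, caches it and runs only TestProgressCurrentStage; the other five tests are unwired.
; Each test adds its own sample quest, then queries it.
; The active test attempts four stage progressions, with its requirement-changing calls disconnected.
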(event `self.ReceiveBeginPlay`
  (`parent.ReceiveBeginPlay`)
  (bind _journal (message `/Game/Journal/BPI_JournalHandler.GetJournal` (`GameplayStatics.GetPlayerCharacter` 0)))
  (bind _output_get (set `self.Journal_0` _journal))
  (`self.TestProgressCurrentStage` _output_get))