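; Dialogue component for MyNPC that extends a parent dialogue class, with placeholder content for the NPC's conversation and quest.
; BeginPlay registers the NPC as quest giver in the journal with a single empty "None" stage, while Dialogue only calls its parent.
; The AddDialogueFast macro wraps AddDialogue, either posting an option-less line or passing up to ten options, audio and animation, then branching execution on the chosen option or update state.
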(event `self.ReceiveBeginPlay`
  (`parent.ReceiveBeginPlay`)
  (bind _journal (`self.GetJournal`))
  (`/Game/Journal/AC_Journal.AddQuest` _journal (`self.NPCName`) "" "" (`|MakeArray` (make `/Game/Journal/Struct_QuestStage` "None" "" (`|MakeMap` "None" :!type "Name"))) "NewEnumerator0"))

(fn `Dialogue`
  (`parent.Dialogue`))