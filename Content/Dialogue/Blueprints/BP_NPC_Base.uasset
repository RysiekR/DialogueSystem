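; BP_NPC_Base is a base NPC Blueprint for the dialogue system, providing a name label and interaction hooks.
; The construction script fills the label from CharacterName, and SetInteractableState shows or hides it.
; ConversationClosed forwards a ConversationClosedMessage to the stored InteractInstigator, which is also exposed through a getter.
; Interact is an empty event, and this graph never assigns InteractInstigator.
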(event `/Game/Dialogue/Blueprints/BPI_Interactable.SetInteractableState`
  (params (`bCanShowInteract?` :type Boolean))
  (if `bCanShowInteract?`
    (`SceneComponent.SetVisibility` (`self.Txt_CharacterName`) true false)
    (else
      (`SceneComponent.SetVisibility` (`self.Txt_CharacterName`) false false))))

(event `/Game/Dialogue/Blueprints/BPI_Interactable.ConversationClosed`
  (message `/Game/Dialogue/Blueprints/BPI_Interactable.ConversationClosed` (`self.InteractInstigator`)))

(event `/Game/Dialogue/Blueprints/BPI_Interactable.Interact`
  (params (Intigator :type "Actor Object Reference")))

(fn `GetInteractInstigator`
  (returns (Instigator :type "Actor Object Reference"))
  (return (`self.InteractInstigator`)))

(fn `UserConstructionScript`
  (`TextRenderComponent.K2_SetText` (`self.Txt_CharacterName`) (`self.CharacterName`)))